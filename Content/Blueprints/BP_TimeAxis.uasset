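; BP_TimeAxis is an unfinished actor for an axis of BP_TimeTick markers meant to track a followed actor's Z position.
; BeginPlay spawns the visible number of ticks at its own transform, but the step storing them in TickActors is disconnected.
; UpdateAxis derives a centred start index from the followed actor's height and tick spacing, but its loop moves nothing and nothing here calls it.
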(event EventBeginPlay
  (for _index (range 0 (Math|Conversions|ToInteger(Byte) (- (Variables|Default|GetVisibleTickCount) 1)))
    (bind _returnvalue (Game|SpawnActorfromClass "/Game/Blueprints/BP_TimeTick.BP_TimeTick_C" (Transformation|GetActorTransform) "Undefined" "MultiplyWithRoot" 0 0))))

(event Collision|EventActorBeginOverlap
  (params (OtherActor :type Actor%20Object%20Reference)))

(event EventTick
  (params (DeltaSeconds :type Float%20%28single-precision%29)))

(fn ConstructionScript)

(fn UpdateAxis
  (bind _followactor (Variables|Default|GetFollowActor))
  (if (Utilities|IsValid _followactor)
    (Variables|Default|SetCenterTickIndex (Class|KismetMathLibrary|FFloor64 (/ (.Z (Math|Vector|BreakVector (Transformation|GetActorLocation _followactor))) (Variables|Default|GetTickSpacing))))
    (Variables|Default|SetStartTickIndex (- (Variables|Default|GetCenterTickIndex) (/ (Variables|Default|GetVisibleTickCount) 2)))
    (for _index (range 0 (- (Utilities|Array|Length (Variables|Default|GetTickActors)) 1))
      _)))